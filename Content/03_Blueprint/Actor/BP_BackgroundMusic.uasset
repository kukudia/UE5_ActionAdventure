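; BP_BackgroundMusic is an actor that plays background music tracks one after another in a loop.
; On BeginPlay, Play sets the current BGMArray track on the Audio component, fades it in and prints the component's name.
; When audio finishes, the index advances, wrapping to zero at the end, and Play runs again.
; The Delay on wrap does not hold up playback, as the Sequence calls Play immediately.
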(event `self.ReceiveBeginPlay`
  (`self.Play`))

(event `self.Audio.OnAudioFinished`
  (`|ExecutionSequence`
    (:`then_0`
      (bind _result (`/Engine/EditorBlueprintResources/StandardMacros.IncrementInt` (`self.BGMIndex`))
        (:`  `
          (if (>= _result (`KismetArrayLibrary.Array_Length` (`self.BGMArray`)))
            (set `self.BGMIndex` 0)
            (`KismetSystemLibrary.Delay` 1.0)))))
    (:`then_1`
      (`self.Play`))))

(fn `Play`
  (bind _audio (`self.Audio`))
  (`AudioComponent.SetSound` _audio (`|GetArrayItem` (`self.BGMArray`) (`self.BGMIndex`)))
  (`AudioComponent.FadeIn` _audio (`self.FadeInTime`) 1.0 0.0 "Linear")
  (`AudioComponent.FadeIn` _audio (`self.FadeInTime`) 1.0 0.0 "Linear")
  (`KismetSystemLibrary.PrintString` (`KismetSystemLibrary.GetDisplayName` _audio) true true (struct :`G` 0.66 :`B` 1.0 :`A` 1.0) 10.0))

(fn `UserConstructionScript`)