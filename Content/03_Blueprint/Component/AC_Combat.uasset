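; Player combat component that implements lock-on targeting for BP_Player.
; The IA_Lock input toggles the lock, sphere-tracing for Pawns along the camera's forward vector and storing the hit actor.
; While locked, Tick turns control rotation toward the target with a downward pitch offset, and character movement follows controller rotation instead of movement direction.
; A BP_TargetLockWidget actor attaches to the target and is destroyed on unlock.
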(event `self.ReceiveBeginPlay`
  (bind _asbp_player (cast `/Game/03_Blueprint/BP_Player` (`self.GetOwner`)))
  (set `self.BP Player` _asbp_player))

(event `self.ReceiveTick`
  (params (DeltaSeconds :type "Float (single-precision)"))
  (bind _bp_player (`self.BP Player`))
  (bind (_returnvalue_roll _returnvalue_pitch _returnvalue_yaw) (`KismetMathLibrary.BreakRotator` (`KismetMathLibrary.FindLookAtRotation` (`Actor.K2_GetActorLocation` _bp_player) (`Actor.K2_GetActorLocation` (`self.TargetLockActor`)))))
  (`self.TargetLockActor`
    (:`then`
      (`Controller.SetControlRotation` (`Pawn.GetController` _bp_player) (`KismetMathLibrary.MakeRotator` _returnvalue_roll (- _returnvalue_pitch 20.0) _returnvalue_yaw)))
    (:`else`)))

(event `EnhancedInput|/Game/Input/Actions/IA_Lock`
  (params (ActionValue :type Boolean) (ElapsedSeconds :type "Float (double-precision)") (TriggeredSeconds :type "Float (double-precision)") (InputAction :type "InputAction Object Reference" :default "/Game/Input/Actions/IA_Lock.IA_Lock"))
  (bind _returnvalue (`Actor.GetTransform` (`self.TargetLockActor`)))
  (bind _transformcomponent (`PlayerCameraManager.TransformComponent` (`GameplayStatics.GetPlayerCameraManager` 0)))
  (bind _charactermovement (`Character.CharacterMovement` (`self.BP Player`)))
  (bind _charactermovement_2 (`Character.CharacterMovement` (`self.BP Player`)))
  (bind (_returnvalue_x _returnvalue_y _returnvalue_z) (`KismetMathLibrary.BreakVector` (`SceneComponent.K2_GetComponentLocation` _transformcomponent)))
  (bind _returnvalue_2 (`KismetMathLibrary.MakeVector` _returnvalue_x _returnvalue_y (+ _returnvalue_z 20.0)))
  (:`Started`
    (`self.TargetLockActor`
      (:`then`
        (set `self.TargetLockActor` null)
        (set `CharacterMovementComponent.bOrientRotationToMovement` true _charactermovement)
        (set `CharacterMovementComponent.bUseControllerDesiredRotation` false _charactermovement)
        (bind _targetlockwidget (`self.TargetLockWidget`)
          (:`then`
            (`Actor.K2_DestroyActor` _targetlockwidget))
          (:`else`)))
      (:`else`
        (bind (_outhit _returnvalue_3) (`KismetSystemLibrary.SphereTraceSingleForObjects` :`Start` _returnvalue_2 :`End` (+ _returnvalue_2 (* (`KismetMathLibrary.GetForwardVector` (`SceneComponent.K2_GetComponentRotation` _transformcomponent)) 1000.0)) :`Radius` 150.0 :`ObjectTypes` (`|MakeArray` "ObjectTypeQuery3" :!type "EObjectTypeQuery Enum") :`DrawDebugType` "ForDuration"))
        (if _returnvalue_3
          (set `self.TargetLockActor` (`.HitActor` (`GameplayStatics.BreakHitResult` _outhit)))
          (set `CharacterMovementComponent.bOrientRotationToMovement` false _charactermovement_2)
          (set `CharacterMovementComponent.bUseControllerDesiredRotation` true _charactermovement_2)
          (bind _returnvalue_4 (`|SpawnActorFromClass` "/Game/03_Blueprint/Actor/BP_TargetLockWidget.BP_TargetLockWidget_C" (`KismetMathLibrary.MakeTransform` (`KismetMathLibrary.MakeVector` (.x (.location _returnvalue)) (.y (.location _returnvalue)) (+ (.z (.location _returnvalue)) 20.0)) (.rotation _returnvalue)) "Undefined" "MultiplyWithRoot" null null))
          (bind _output_get (set `self.TargetLockWidget` _returnvalue_4))
          (`Actor.K2_AttachToActor` _output_get (`self.TargetLockActor`) "None" "SnapToTarget" "SnapToTarget" "SnapToTarget" true))))))