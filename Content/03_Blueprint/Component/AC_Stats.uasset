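; AC_Stats is an actor component that tracks its owner's health.
; UpdateHealthValue adds a signed value to Health, prints the result, and calls Die at zero or below, which sends DieMessage to the owner.
; It also sets a progress bar, supplied through SetHealthProgressBar, to the Health to MaxHealth ratio when that bar is valid.
; Health is not clamped, so Die can fire again on later updates.
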(event `Die`
  (message `/Game/03_Blueprint/Interface/I_Blade.Die` (`self.GetOwner`)))

(event `SetHealthProgressBar`
  (params (HealthProgressBar :type "ProgressBar Object Reference"))
  (set `self.Health Progress Bar` HealthProgressBar))

(fn `UpdateHealthValue`
  (params (Stat :type "/Game/03_Blueprint/Enum/E_Stats Enum" :default "NewEnumerator0") (Value :type "Float (double-precision)"))
  (bind _returnvalue (+ (`self.Health`) Value))
  (switch `/Game/03_Blueprint/Enum/E_Stats` Stat
    (:`NewEnumerator0`
      (`KismetSystemLibrary.PrintString` (`KismetStringLibrary.Conv_DoubleToString` _returnvalue))
      (set `self.Health` _returnvalue)
      (`|ExecutionSequence`
        (:`then_0`
          (if (<= (`self.Health`) 0.0)
            (`self.Die`)))
        (:`then_1`
          (bind _health_progress_bar (`self.Health Progress Bar`)
            (:`then`
              (`ProgressBar.SetPercent` _health_progress_bar (/ (`self.Health`) (`self.MaxHealth`))))
            (:`else`)))))))