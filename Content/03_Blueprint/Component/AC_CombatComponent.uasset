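; Player combat component for BP_Player, handling target lock, left and right attacks, directional dodge and weapon damage.
; An enum state gates actions and, with lock status, drives rotation mode and walk speed.
; Lock sphere-traces from the camera, attaches a marker actor and steers control rotation until out of range.
; Damage start/end events run a looping timer sphere trace with throttled hits and spawn cycling blade Niagara effects.
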(event `self.ReceiveBeginPlay`
  ; BeginPlay
  (bind _asbp_player (cast `/Game/03_Blueprint/BP_Player` (`self.GetOwner`)))
  (set `self.BP Player` _asbp_player)
  (set `self.PlayerStates` "NewEnumerator3")
  (`self.OnStateChanged`))

(event `self.ReceiveTick`
  (params (DeltaSeconds :type "Float (single-precision)"))
  (bind _bp_player (`self.BP Player`))
  (bind (_returnvalue_roll _returnvalue_pitch _returnvalue_yaw) (`KismetMathLibrary.BreakRotator` (`KismetMathLibrary.FindLookAtRotation` (`Actor.K2_GetActorLocation` _bp_player) (`Actor.K2_GetActorLocation` (`self.TargetLockActor`)))))
  ; Tick
  (if (not (`self.isDead`))
    (`self.DebugStates`)
    (bind _targetlockactor (`self.TargetLockActor`)
      (:`then`
        (if (< (`Actor.GetDistanceTo` _targetlockactor _bp_player) 1500.0)
          (`Controller.SetControlRotation` (`Pawn.GetController` _bp_player) (`KismetMathLibrary.MakeRotator` _returnvalue_roll (- _returnvalue_pitch 20.0) _returnvalue_yaw))
          (else
            (`self.UnLock`))))
      (:`else`))))

(event `EnhancedInput|/Game/Input/Actions/IA_Lock`
  (params (ActionValue :type Boolean) (ElapsedSeconds :type "Float (double-precision)") (TriggeredSeconds :type "Float (double-precision)") (InputAction :type "InputAction Object Reference" :default "/Game/Input/Actions/IA_Lock.IA_Lock"))
  ; Lock
  (:`Started`
    (`self.TargetLockActor`
      (:`then`
        (`self.UnLock`))
      (:`else`
        (`self.Lock`)))))

(event `EnhancedInput|/Game/Input/Actions/IA_LeftAttack`
  (params (ActionValue :type Boolean) (ElapsedSeconds :type "Float (double-precision)") (TriggeredSeconds :type "Float (double-precision)") (InputAction :type "InputAction Object Reference" :default "/Game/Input/Actions/IA_LeftAttack.IA_LeftAttack"))
  ; Atttack
  (:`Triggered`
    (if (not (`|EnumEquality` (`self.PlayerStates`) "NewEnumerator1"))
      (set `self.PlayerStates` "NewEnumerator1")
      (`self.OnStateChanged`)
      (set `self.LeftAttack` (`|GetArrayItem` (`self.LeftAttackAnim`) (`self.AttackCount`)))
      (bind _leftattack (`self.LeftAttack`)
        (:`then`
          (`|PlayMontage` (`Character.Mesh` (`self.BP Player`)) _leftattack
            (:`then`
              (`KismetSystemLibrary.PrintString` (`KismetStringLibrary.Conv_IntToString` (`self.AttackCount`)))
              (bind _result (`/Engine/EditorBlueprintResources/StandardMacros.IncrementInt` (`self.AttackCount`))
                (:`  `
                  (if (>= _result (`KismetArrayLibrary.Array_Length` (`self.LeftAttackAnim`)))
                    (set `self.AttackCount` 0)))))
            (:`OnBlendOut`
              (set `self.PlayerStates` "NewEnumerator3")
              (`self.OnStateChanged`))))
        (:`else`)))))

(event `EnhancedInput|/Game/Input/Actions/IA_RightAttack`
  (params (ActionValue :type Boolean) (ElapsedSeconds :type "Float (double-precision)") (TriggeredSeconds :type "Float (double-precision)") (InputAction :type "InputAction Object Reference" :default "/Game/Input/Actions/IA_RightAttack.IA_RightAttack"))
  ; Atttack
  (:`Triggered`
    (if (not (`|EnumEquality` (`self.PlayerStates`) "NewEnumerator1"))
      (set `self.PlayerStates` "NewEnumerator1")
      (`self.OnStateChanged`)
      (`|PlayMontage` (`Character.Mesh` (`self.BP Player`)) (`self.RightAttack`)
        (:`then`
          (`KismetSystemLibrary.PrintString` "-1"))
        (:`OnBlendOut`
          (set `self.PlayerStates` "NewEnumerator3")
          (`self.OnStateChanged`))))))

(event `EndDamageTrace`
  ; SwordTrace
  (if (`KismetSystemLibrary.K2_IsValidTimerHandle` (stale `StartDamageTrace` _returnvalue))
    (`KismetSystemLibrary.K2_ClearAndInvalidateTimerHandle` (stale `StartDamageTrace` _returnvalue))
    (`self.DestroyBlade`)))

(event `StartDamageTrace`
  ; SwordTrace
  (bind _returnvalue (`KismetSystemLibrary.K2_SetTimerDelegate` (delegate `DamageTrace`) 0.01 true))
  (`self.SpawnBlade`))

(event `DamageTrace`
  (bind _bp_player (`self.BP Player`))
  ; SwordTrace
  (bind (_outhit _returnvalue) (`KismetSystemLibrary.SphereTraceSingleForObjects` :`Start` (`SceneComponent.K2_GetComponentLocation` (`/Game/03_Blueprint/BP_Player.BladeStartPos` _bp_player)) :`End` (`SceneComponent.K2_GetComponentLocation` (`/Game/03_Blueprint/BP_Player.HurtEndPos` _bp_player)) :`Radius` 30.0 :`ObjectTypes` (`|MakeArray` "ObjectTypeQuery3" :!type "EObjectTypeQuery Enum") :`DrawDebugType` "ForOneFrame"))
  (if _returnvalue
    (`/Engine/EditorBlueprintResources/StandardMacros.DoOnce` false :!label _label
      (:`Completed`
        (`GameplayStatics.ApplyDamage` (`.HitActor` (`GameplayStatics.BreakHitResult` _outhit)) (`self.Base Damage`))
        (`KismetSystemLibrary.Delay` 0.2)
        (goto _label :!via `Reset`)))))

(event `EnhancedInput|/Game/Input/Actions/IA_Dodge`
  (params (ActionValue :type Boolean) (ElapsedSeconds :type "Float (double-precision)") (TriggeredSeconds :type "Float (double-precision)") (InputAction :type "InputAction Object Reference" :default "/Game/Input/Actions/IA_Dodge.IA_Dodge"))
  (bind _bp_player (`self.BP Player`))
  (:`Started`
    (if (not (`|EnumEquality` (`self.PlayerStates`) "NewEnumerator2"))
      (set `self.PlayerStates` "NewEnumerator2")
      (`self.OnStateChanged`)
      (`|ExecutionSequence`
        (:`then_0`
          (if (`CharacterMovementComponent.bUseControllerDesiredRotation` (`Character.CharacterMovement` _bp_player))
            (switch `string` (`KismetTextLibrary.Conv_TextToString` (`KismetInputLibrary.Key_GetDisplayName` (`/Game/03_Blueprint/BP_Player.Direction Key` _bp_player)))
              (:`Default`
                (set `self.MovementDir` "NewEnumerator0"))
              (:`W`
                (set `self.MovementDir` "NewEnumerator0"))
              (:`A`
                (set `self.MovementDir` "NewEnumerator1"))
              (:`S`
                (set `self.MovementDir` "NewEnumerator2"))
              (:`D`
                (set `self.MovementDir` "NewEnumerator3")))
            (else
              (set `self.MovementDir` "NewEnumerator0"))))
        (:`then_1`
          (`AudioComponent.Play` (`/Game/03_Blueprint/BP_Player.DodgeSound` (`self.BP Player`)) 0.0)
          (`|PlayMontage` (`Character.Mesh` (`self.BP Player`)) (select `/Game/03_Blueprint/Enum/E_MovementDir` (`self.MovementDir`) :`NewEnumerator0` "/Game/01_Animation/SpearAnimation/Animation/Dodge/Anim_Dodge_F_Montage.Anim_Dodge_F_Montage" :`NewEnumerator1` "/Game/01_Animation/SpearAnimation/Animation/Dodge/Anim_Dodge_L_Montage.Anim_Dodge_L_Montage" :`NewEnumerator2` "/Game/01_Animation/SpearAnimation/Animation/Dodge/Anim_Dodge_B_Montage.Anim_Dodge_B_Montage" :`NewEnumerator3` "/Game/01_Animation/SpearAnimation/Animation/Dodge/Anim_Dodge_R_Montage.Anim_Dodge_R_Montage" :!type "AnimMontage Object Reference")
            (:`OnBlendOut`
              (set `self.PlayerStates` "NewEnumerator3")
              (`self.OnStateChanged`))
            (:`OnInterrupted`
              (`AudioComponent.FadeOut` (`/Game/03_Blueprint/BP_Player.DodgeSound` (`self.BP Player`)) 0.5 0.0 "Linear"))))))))

(event `OnStateChanged`
  (bind _charactermovement (`Character.CharacterMovement` (`self.BP Player`)))
  (bind _charactermovement_2 (`Character.CharacterMovement` (`self.BP Player`)))
  (if (not (`|EnumEquality` (`self.PlayerStates`) "NewEnumerator5"))
    (`|ExecutionSequence`
      (:`then_0`
        (if (or (`self.isLocking`) (`|EnumEquality` (`self.PlayerStates`) "NewEnumerator1"))
          (set `CharacterMovementComponent.bUseControllerDesiredRotation` true _charactermovement_2)
          (set `CharacterMovementComponent.bOrientRotationToMovement` false _charactermovement_2)
          (else
            (set `CharacterMovementComponent.bUseControllerDesiredRotation` false _charactermovement_2)
            (set `CharacterMovementComponent.bOrientRotationToMovement` true _charactermovement_2))))
      (:`then_1`
        (if (`|EnumEquality` (`self.PlayerStates`) "NewEnumerator4")
          (set `CharacterMovementComponent.MaxWalkSpeed` 0.0 _charactermovement)
          (else
            (set `CharacterMovementComponent.MaxWalkSpeed` 480.0 _charactermovement)))))))

(fn `DebugStates`
  (bind _charactermovement (`Character.CharacterMovement` (`self.BP Player`)))
  (`|ExecutionSequence`
    (:`then_0`
      (if (`self.isLocking`)
        (`KismetSystemLibrary.PrintString` "Lock" true true (struct :`G` 0.66 :`B` 1.0 :`A` 1.0) 0.0)
        (else
          (`KismetSystemLibrary.PrintString` "Lock" true true (struct :`R` 1.0 :`A` 1.0) 0.0))))
    (:`then_1`
      (if (`CharacterMovementComponent.bOrientRotationToMovement` _charactermovement)
        (`KismetSystemLibrary.PrintString` "OrientRotation" true true (struct :`G` 0.66 :`B` 1.0 :`A` 1.0) 0.0)))
    (:`then_2`
      (if (`CharacterMovementComponent.bUseControllerDesiredRotation` _charactermovement)
        (`KismetSystemLibrary.PrintString` "ControllerDesiredRotation" true true (struct :`G` 0.66 :`B` 1.0 :`A` 1.0) 0.0)))
    (:`then_3`
      (`KismetSystemLibrary.PrintString` (`|GetEnumeratorNameAsString` (`self.PlayerStates`)) true true (struct :`R` 1.0 :`G` 1.0 :`B` 1.0 :`A` 1.0) 0.0))))

(fn `DestroyBlade`
  (bind _fx (`self.FX`)
    (:`then`
      (`self.K2_DestroyComponent` _fx)
      (bind _result (`/Engine/EditorBlueprintResources/StandardMacros.IncrementInt` (`self.ParticleCount`))
        (:`  `
          (if (>= _result (`KismetArrayLibrary.Array_Length` (`self.BladeFXSet`)))
            (set `self.ParticleCount` 0)))))
    (:`else`)))

(fn `Lock`
  (bind _returnvalue (`Actor.GetTransform` (`self.TargetLockActor`)))
  (bind _transformcomponent (`PlayerCameraManager.TransformComponent` (`GameplayStatics.GetPlayerCameraManager` 0)))
  (bind _charactermovement (`Character.CharacterMovement` (`self.BP Player`)))
  (bind (_returnvalue_x _returnvalue_y _returnvalue_z) (`KismetMathLibrary.BreakVector` (`SceneComponent.K2_GetComponentLocation` _transformcomponent)))
  (bind _returnvalue_2 (`KismetMathLibrary.MakeVector` _returnvalue_x _returnvalue_y (+ _returnvalue_z 20.0)))
  (bind (_outhit _returnvalue_3) (`KismetSystemLibrary.SphereTraceSingleForObjects` :`Start` _returnvalue_2 :`End` (+ _returnvalue_2 (* (`KismetMathLibrary.GetForwardVector` (`SceneComponent.K2_GetComponentRotation` _transformcomponent)) 1500.0)) :`Radius` 300.0 :`ObjectTypes` (`|MakeArray` "ObjectTypeQuery3" :!type "EObjectTypeQuery Enum") :`DrawDebugType` "ForDuration"))
  (if _returnvalue_3
    (set `self.TargetLockActor` (`.HitActor` (`GameplayStatics.BreakHitResult` _outhit)))
    (set `CharacterMovementComponent.bOrientRotationToMovement` false _charactermovement)
    (set `CharacterMovementComponent.bUseControllerDesiredRotation` true _charactermovement)
    (bind _returnvalue_4 (`|SpawnActorFromClass` "/Game/03_Blueprint/Actor/BP_TargetLockWidget.BP_TargetLockWidget_C" (`KismetMathLibrary.MakeTransform` (`KismetMathLibrary.MakeVector` (.x (.location _returnvalue)) (.y (.location _returnvalue)) (+ (.z (.location _returnvalue)) 20.0)) (.rotation _returnvalue)) "Undefined" "MultiplyWithRoot" null null))
    (bind _output_get (set `self.TargetLockWidget` _returnvalue_4))
    (bind _returnvalue_5 (`Actor.K2_AttachToActor` _output_get (`self.TargetLockActor`) "None" "SnapToTarget" "SnapToTarget" "SnapToTarget" true))
    (set `self.isLocking` _returnvalue_5)))

(fn `SpawnBlade`
  (bind _bp_player (`self.BP Player`))
  (bind _returnvalue (`SceneComponent.K2_GetComponentLocation` (`/Game/03_Blueprint/BP_Player.BladeStartPos` _bp_player)))
  (bind _returnvalue_2 (`SceneComponent.K2_GetComponentLocation` (`/Game/03_Blueprint/BP_Player.BladeEndPos` _bp_player)))
  (`self.FX`
    (:`then`)
    (:`else`
      (set `self.BladeFX` (`|GetArrayItem` (`self.BladeFXSet`) (`self.ParticleCount`)))
      (bind _bladefx (`self.BladeFX`)
        (:`then`
          (bind _returnvalue_3 (`NiagaraFunctionLibrary.SpawnSystemAttached` _bladefx (`/Game/03_Blueprint/BP_Player.Spear` (`self.BP Player`)) "None" (/ (+ _returnvalue _returnvalue_2) 2) (`KismetMathLibrary.MakeRotFromX` (- _returnvalue _returnvalue_2)) "KeepWorldPosition"))
          (set `self.FX` _returnvalue_3))
        (:`else`)))))

(fn `UnLock`
  (bind _charactermovement (`Character.CharacterMovement` (`self.BP Player`)))
  (set `self.TargetLockActor` null)
  (set `CharacterMovementComponent.bOrientRotationToMovement` true _charactermovement)
  (set `CharacterMovementComponent.bUseControllerDesiredRotation` false _charactermovement)
  (bind _targetlockwidget (`self.TargetLockWidget`)
    (:`then`
      (`Actor.K2_DestroyActor` _targetlockwidget)
      (set `self.isLocking` false))
    (:`else`)))