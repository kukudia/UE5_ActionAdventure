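; Base river-tool prefab Blueprint that builds spline meshes along its child spline components in the construction script.
; Each spline is matched by component name to a Splines entry, whose enabled settings feed GenerateSplineMesh; unmatched splines get no mesh.
; GenerateSplineMesh places segments at fixed distance spacing, applying offset and deriving roll and scale from the spline.
; Auto-registering default settings for new splines exists only in unconnected graph logic.
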(fn `GenerateSplineMesh`
  (params (Collision :type "ECollisionEnabled Enum" :default "NoCollision") (CastShadow :type Boolean) (Material :type "MaterialInterface Object Reference") (TargetSpline :type "SplineComponent Object Reference") (SplineStartOffset :type "Float (double-precision)") (Offset :type "Vector Structure") (Scale :type "Vector Structure") (TangetScale :type "Float (double-precision)") (Spacing :type "Float (double-precision)") (Rotation :type "Rotator Structure") (StaticMesh :type "StaticMesh Object Reference"))
  (bind _y (.y Scale))
  (bind _z (.z Scale))
  (for _index (range (+ (`.ReturnValue` (`KismetMathLibrary.FMod` (`SplineComponent.GetSplineLength` TargetSpline) Spacing)) 1))
    (bind _returnvalue (`AddComponent|NODE_AddSplineMeshComponent-2` :`bManualAttachment` true :`RelativeTransform` (`KismetMathLibrary.MakeTransform` (0.0 0.0 0.0) Rotation)))
    (`PrimitiveComponent.SetCollisionEnabled` _returnvalue Collision)
    (`PrimitiveComponent.SetCastShadow` _returnvalue CastShadow)
    (`StaticMeshComponent.SetStaticMesh` _returnvalue StaticMesh)
    (`PrimitiveComponent.SetMaterial` _returnvalue 0 Material)
    (bind _returnvalue_2 (* _index Spacing))
    (bind _returnvalue_3 (+ SplineStartOffset _returnvalue_2))
    (bind _returnvalue_4 (+ (+ _returnvalue_2 Spacing) SplineStartOffset))
    (`SplineMeshComponent.SetStartAndEnd` _returnvalue (+ (+ (`SplineComponent.GetLocationAtDistanceAlongSpline` TargetSpline _returnvalue_3 "World") (* Offset (- (`KismetMathLibrary.MakeVector` 1.0 (.y (`SplineComponent.GetScaleAtDistanceAlongSpline` TargetSpline _returnvalue_3)) (.z (`SplineComponent.GetScaleAtDistanceAlongSpline` TargetSpline _returnvalue_3))) (1.0 1.0 1.0)))) (`KismetMathLibrary.GreaterGreater_VectorRotator` Offset (`SplineComponent.GetRotationAtDistanceAlongSpline` TargetSpline _returnvalue_3 "Local"))) (* (`SplineComponent.GetDirectionAtDistanceAlongSpline` TargetSpline _returnvalue_3 "World") TangetScale) (+ (+ (* Offset (- (`KismetMathLibrary.MakeVector` 1.0 (.y (`SplineComponent.GetScaleAtDistanceAlongSpline` TargetSpline _returnvalue_4)) (.z (`SplineComponent.GetScaleAtDistanceAlongSpline` TargetSpline _returnvalue_4))) (1.0 1.0 1.0))) (`SplineComponent.GetLocationAtDistanceAlongSpline` TargetSpline _returnvalue_4 "World")) (`KismetMathLibrary.GreaterGreater_VectorRotator` Offset (`SplineComponent.GetRotationAtDistanceAlongSpline` TargetSpline _returnvalue_4 "Local"))) (* (`SplineComponent.GetDirectionAtDistanceAlongSpline` TargetSpline _returnvalue_4 "World") TangetScale) true)
    (bind _returnvalue_5 (* Spacing (`KismetMathLibrary.Conv_IntToDouble` _index)))
    (bind _returnvalue_6 (+ _returnvalue_5 (* Spacing 0.5)))
    (`SplineMeshComponent.SetSplineUpDir` _returnvalue (`SplineComponent.GetUpVectorAtDistanceAlongSpline` TargetSpline _returnvalue_6 "World") true)
    (bind _returnvalue_7 (`KismetMathLibrary.NegateRotator` (`SplineComponent.GetRotationAtDistanceAlongSpline` TargetSpline _returnvalue_6 "World")))
    (`SplineMeshComponent.SetStartRoll` _returnvalue (`KismetMathLibrary.DegreesToRadians` (.roll (`KismetMathLibrary.ComposeRotators` (`SplineComponent.GetRotationAtDistanceAlongSpline` TargetSpline _returnvalue_5 "World") _returnvalue_7))) true)
    (bind _returnvalue_8 (+ _returnvalue_5 Spacing))
    (`SplineMeshComponent.SetEndRoll` _returnvalue (`KismetMathLibrary.DegreesToRadians` (.roll (`KismetMathLibrary.ComposeRotators` (`SplineComponent.GetRotationAtDistanceAlongSpline` TargetSpline _returnvalue_8 "World") _returnvalue_7))) true)
    (`SplineMeshComponent.SetStartScale` _returnvalue (`KismetMathLibrary.MakeVector2D` (* (.y (`SplineComponent.GetScaleAtDistanceAlongSpline` TargetSpline _returnvalue_5)) _y) (* (.z (`SplineComponent.GetScaleAtDistanceAlongSpline` TargetSpline _returnvalue_5)) _z)) true)
    (`SplineMeshComponent.SetEndScale` _returnvalue (`KismetMathLibrary.MakeVector2D` (* _y (.y (`SplineComponent.GetScaleAtDistanceAlongSpline` TargetSpline _returnvalue_8))) (* (.z (`SplineComponent.GetScaleAtDistanceAlongSpline` TargetSpline _returnvalue_8)) _z)) true)))

(fn `UserConstructionScript`
  (bind _splines (`self.Splines`))
  (bind (_riversplinemesh _splinematerial _spacing _scale _offset _rotation _tangetscale _splinestartoffset _collisiontype _castshadow _enabled) (break `/Game/UltimateRiverTool/Blueprints/Structures/RiverSplineElement` (`self.CurrentSplineProperties`)))
  (`KismetMathLibrary.SetRandomStreamSeed` (`self.RandomStream`) (`self.RandomSeed`))
  (for _array_element (`SceneComponent.GetChildrenComponents` (`self.DefaultSceneRoot`) true)
    (if (== (`GameplayStatics.GetObjectClass` _array_element) "/Script/Engine.SplineComponent")
      (bind `_as样条组件` (cast `SplineComponent` _array_element))
      (set `self.CurrentSpline` `_as样条组件`)
      (`KismetArrayLibrary.Array_Add` (`self.debug`) (`KismetStringLibrary.Conv_IntToString` (`KismetArrayLibrary.Array_Length` _splines)))
      (for _array_element_2 _splines
        (bind (_splinename _splineproperties) (break `/Game/UltimateRiverTool/Blueprints/Structures/SplinesInEditor` _array_element_2))
        (set `self.CurrentSplineProperties` _splineproperties)
        (if (`KismetStringLibrary.EqualEqual_StrStr` _splinename (`KismetSystemLibrary.GetObjectName` _array_element))
          (`|ExecutionSequence`
            (:`then_0`
              (if (!= _riversplinemesh null)
                (if _enabled
                  (`self.GenerateSplineMesh` _collisiontype _castshadow _splinematerial (`self.CurrentSpline`) _splinestartoffset _offset _scale _tangetscale _spacing _rotation _riversplinemesh))))
            (:`then_1`
              (break))))))))