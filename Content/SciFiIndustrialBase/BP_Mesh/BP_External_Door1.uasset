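; Automatic two-panel external door that opens on overlap with its Box trigger and closes after a delay, with sounds for each direction.
; One timeline slides and slightly angles both panels while counter-rotating the two rollers, and plays in reverse to close.
; Flags derived from the timeline's position drive a web of gates, a DoOnce and a retriggerable delay to handle entering or leaving mid-motion.
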(event `self.Box.OnComponentBeginOverlap`
  (params (OverlappedComponent :type "PrimitiveComponent Object Reference") (OtherActor :type "Actor Object Reference") (OtherComp :type "PrimitiveComponent Object Reference") (OtherBodyIndex :type Integer) (bFromSweep :type Boolean) (SweepResult :type "HitResult Structure (by ref)"))
  (bind _returnvalue (`self.K2_GetActorLocation`))
  (`|ExecutionSequence`
    (:`then_0`
      (if (not (`self.Open`))
        (`GameplayStatics.PlaySoundAtLocation` "/Game/SciFiIndustrialBase/Sound/SC_Open_Door_2_Cue.SC_Open_Door_2_Cue" _returnvalue (struct) 1.0 1.0 0.0 null null null null :!label _label)
        (bind (_direction _newtrack_0) (`Timeline|Timeline_0` :!label _label_2)
          (:`Update`
            (bind _returnvalue_2 (`KismetMathLibrary.Lerp` 0.0 450.0 _newtrack_0))
            (set `self.Close` (> _returnvalue_2 445.0))
            (set `self.Open` (< 0.0 _newtrack_0))
            (set `self.NewVar_2` (< (`KismetMathLibrary.Lerp` 445.0 0.0 _newtrack_0) 445.0))
            (set `self.NewVar_3` (> (`KismetMathLibrary.Lerp` 0.0 -450.0 _newtrack_0) -450.0))
            (`|ExecutionSequence`
              (:`then_0`
                (`SceneComponent.K2_SetRelativeLocationAndRotation` (`self.RightDoor`) (`KismetMathLibrary.MakeVector` (`KismetMathLibrary.Lerp` 100.0 91.0 _newtrack_0) (`KismetMathLibrary.Lerp` 0.0 -450.0 _newtrack_0) 50.0) (`KismetMathLibrary.MakeRotator` 0.0 0.0 (`KismetMathLibrary.Lerp` -90.0 -93.5 _newtrack_0)) false false))
              (:`then_1`
                (`SceneComponent.K2_SetRelativeLocationAndRotation` (`self.LeftDoor`) (`KismetMathLibrary.MakeVector` (`KismetMathLibrary.Lerp` 100.0 91.0 _newtrack_0) _returnvalue_2 50.0) (`KismetMathLibrary.MakeRotator` 0.0 0.0 (`KismetMathLibrary.Lerp` -90.0 -86.0 _newtrack_0)) false false))
              (:`then_2`
                (`SceneComponent.K2_SetRelativeRotation` (`self.Roller right`) (`KismetMathLibrary.MakeRotator` 0.0 0.0 (`KismetMathLibrary.Lerp` 0.0 360.0 _newtrack_0)) false false))
              (:`then_3`
                (`SceneComponent.K2_SetRelativeRotation` (`self.Roller left`) (`KismetMathLibrary.MakeRotator` 0.0 0.0 (`KismetMathLibrary.Lerp` 0.0 -360.0 _newtrack_0)) false false))))
          (:`Finished`
            (set `self.Close` (> _returnvalue_2 445.0))
            (`|ExecutionSequence`
              (:`then_0`
                (if (`self.NewVar_3`)
                  (`/Engine/EditorBlueprintResources/StandardMacros.Gate` true :!label _label_3
                    (:`Exit`
                      (`KismetSystemLibrary.Delay` 2.0)
                      (`/Engine/EditorBlueprintResources/StandardMacros.Gate` true :!label _label_4
                        (:`Exit`
                          (goto _label)))))
                  (else
                    (`/Engine/EditorBlueprintResources/StandardMacros.Gate` true :!label _label_5
                      (:`Exit`
                        (if (`self.NewVar_2`) :!label _label_6
                          (`KismetSystemLibrary.RetriggerableDelay` 4.0 :!label _label_7)
                          (`|ExecutionSequence`
                            (:`then_0`
                              (`/Engine/EditorBlueprintResources/StandardMacros.Gate` true :!label _label_8
                                (:`Exit`
                                  (`GameplayStatics.PlaySoundAtLocation` "/Game/SciFiIndustrialBase/Sound/SC_Close_Door_2_Cue.SC_Close_Door_2_Cue" _returnvalue (struct) 1.0 1.0 0.0 null null null null)
                                  (goto _label_2 :!via `Reverse`))))
                            (:`then_1`
                              (goto _label_5 :!via `Close`))
                            (:`then_2`
                              (goto _label_4 :!via `Open`)))))))))
              (:`then_1`
                (if (`self.NewVar_1`)
                  (`/Engine/EditorBlueprintResources/StandardMacros.DoOnce` false :!label _label_9
                    (:`Completed`
                      (`|ExecutionSequence`
                        (:`then_0`
                          (goto _label_6))
                        (:`then_1`
                          (goto _label_8 :!via `Open`)))))))
              (:`then_2`
                (goto _label_3 :!via `Close`))
              (:`then_3`
                (if (not (`self.NewVar_2`))
                  (goto _label_8 :!via `Close`))))))))
    (:`then_1`
      (goto _label_3 :!via `Open`))
    (:`then_2`
      (if (`self.NewVar_2`)
        (goto _label_8 :!via `Close`)))))

(event `self.Box.OnComponentEndOverlap`
  (params (OverlappedComponent :type "PrimitiveComponent Object Reference") (OtherActor :type "Actor Object Reference") (OtherComp :type "PrimitiveComponent Object Reference") (OtherBodyIndex :type Integer))
  (set `self.NewVar_1` (> (`KismetMathLibrary.Lerp` 0.0 -450.0 (stale `self.Box.OnComponentBeginOverlap` _newtrack_0)) -445.0))
  (`|ExecutionSequence`
    (:`then_0`
      (if (`self.Close`)
        (`|ExecutionSequence`
          (:`then_0`
            (goto _label_7))
          (:`then_1`
            (goto _label_8 :!via `Open`)))
        (else
          (goto _label_9 :!via `Reset`))))
    (:`then_1`
      (goto _label_5 :!via `Open`))
    (:`then_2`
      (goto _label_4 :!via `Close`))))

(fn `UserConstructionScript`)